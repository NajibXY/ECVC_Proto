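; BP_Mechant is an AI-moved pawn that roams the navmesh while spawning trash or fruit projectiles.
; After a startup delay on BeginPlay, it loops: ThrowObject, move to a random navigable point around itself, short pause, repeat, whether the move succeeds or fails.
; ThrowObject randomly picks Trash_Projectile or Fruit_Projectile, spawns it high above the mesh and prints a debug string.
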(event `self.ReceiveBeginPlay`
  (`KismetSystemLibrary.Delay` 5.0)
  (`self.ThrowObject` :!label _label)
  (bind _randomlocation (`NavigationSystemV1.K2_GetRandomLocationInNavigableRadius` (`SceneComponent.K2_GetComponentLocation` (`self.Mesh`)) 3000.0 null null))
  (`|AIMoveTo` self _randomlocation null
    (:`OnSuccess`
      _)
    (:`OnFail`
      _))
  (`KismetSystemLibrary.Delay` 2.0)
  (goto _label))

(fn `ThrowObject`
  (bind _returnvalue (`SceneComponent.K2_GetComponentToWorld` (`self.Mesh`)))
  (bind _returnvalue_2 (`SceneComponent.K2_GetComponentToWorld` (`self.Mesh`)))
  (if (`KismetMathLibrary.RandomBool`)
    (`|SpawnActorFromClass` "/Game/Blueprints/Trash_Projectile.Trash_Projectile_C" (`KismetMathLibrary.MakeTransform` (`KismetMathLibrary.MakeVector` (.x (.location _returnvalue)) (.y (.location _returnvalue)) (+ (.z (.location _returnvalue)) 2000.0))) "Undefined" "MultiplyWithRoot" null null)
    (`KismetSystemLibrary.PrintString` "\"SPAWN TRASH\"")
    (else
      (`|SpawnActorFromClass` "/Game/Blueprints/Fruit_Projectile.Fruit_Projectile_C" (`KismetMathLibrary.MakeTransform` (`KismetMathLibrary.MakeVector` (.x (.location _returnvalue_2)) (.y (.location _returnvalue_2)) (+ (.z (.location _returnvalue_2)) 2000.0))) "Undefined" "MultiplyWithRoot" null null)
      (`KismetSystemLibrary.PrintString` "\"SPAWN FRUIT\""))))

(fn `UserConstructionScript`)