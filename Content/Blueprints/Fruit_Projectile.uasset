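; Fruit projectile actor that changes the game's pollution level when it hits the arena.
; On BeginPlay it caches the GameManager, and on overlapping Arena_Blueprint it applies its Pollution value, spawns an explosion VFX and destroys itself.
; ApplyBonus also changes pollution through the GameManager, scaling the value negatively for a bonus and more heavily positive otherwise.
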(event `self.ReceiveBeginPlay`
  (bind _returnvalue (`GameplayStatics.GetActorOfClass` "/Game/Blueprints/GameManager.GameManager_C"))
  (set `self.GameManager` _returnvalue))

(event `self.ReceiveActorBeginOverlap`
  (params (OtherActor :type "Actor Object Reference"))
  (cast `/Game/Blueprints/Arena_Blueprint` OtherActor)
  (`/Game/Blueprints/GameManager.ChangePollution` (`self.GameManager`) (`self.Pollution`))
  (`KismetSystemLibrary.PrintString` "BOOM FRUIT")
  (`self.Explode`)
  (`self.K2_DestroyActor`))

(event `self.ReceiveTick`
  (params (DeltaSeconds :type "Float (single-precision)")))

(fn `ApplyBonus`
  (params (isBonus :type Boolean))
  (if isBonus
    (`/Game/Blueprints/GameManager.ChangePollution` (`self.GameManager`) (* (`self.Pollution`) -2.0))
    (else
      (`/Game/Blueprints/GameManager.ChangePollution` (`self.GameManager`) (* (`self.Pollution`) 4.0)))))

(fn `Explode`
  (`|SpawnActorFromClass` "/Game/Blueprints/ExplosionFruitVFX.ExplosionFruitVFX_C" (`self.GetTransform`) "Undefined" "MultiplyWithRoot" null null))

(fn `UserConstructionScript`)