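; GameManager actor that tracks a pollution level and shows it through the color of the volumetric clouds.
; On BeginPlay it puts a dynamic material instance on the VolumetricCloud and sets its Albedo to the clean color.
; ChangePollution adds a modifier, clamped only at zero, then blends Albedo toward the full-pollution color by Pollution over 100.
; It also loops over all Platform actors, but the loop body is empty.
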(event `self.ReceiveBeginPlay`
  (bind _volumetriccloud (`self.VolumetricCloud`))
  (bind _returnvalue (`KismetMaterialLibrary.CreateDynamicMaterialInstance` (`VolumetricCloudComponent.Material` _volumetriccloud)))
  (bind _output_get (set `self.CloudMat` _returnvalue))
  (`VolumetricCloudComponent.SetMaterial` _volumetriccloud _returnvalue)
  (`MaterialInstanceDynamic.SetVectorParameterValue` _output_get "Albedo" (`self.NoPollutionColor`)))

(event `self.ReceiveTick`
  (params (DeltaSeconds :type "Float (single-precision)")))

(fn `ChangePollution`
  (params (pollutionModifyer :type "Float (double-precision)"))
  (bind _returnvalue (+ pollutionModifyer (`self.Pollution`)))
  (bind _output_get (set `self.Pollution` (`KismetMathLibrary.FClamp` _returnvalue 0.0 _returnvalue)))
  (bind _returnvalue_2 (/ _output_get 100.0))
  (set `self.PollutionPercent` _returnvalue_2)
  (`MaterialInstanceDynamic.SetVectorParameterValue` (`self.CloudMat`) "Albedo" (`KismetMathLibrary.LinearColorLerp` (`self.NoPollutionColor`) (`self.FullPollutionColor`) _returnvalue_2))
  (bind _outactors (`GameplayStatics.GetAllActorsOfClass` "/Game/Blueprints/Platform.Platform_C"))
  (for _array_element _outactors
    _))

(fn `UserConstructionScript`)